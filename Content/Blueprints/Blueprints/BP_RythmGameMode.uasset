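; Rhythm game mode that loads the chart data for a test song.
; A one-time initializeGame event builds a path from the project directory to a hardcoded JSON file and reads its BPM and Song fields into BPM and NoteArray.
; A failed load prints an error and quits after a short delay.
; A SplitCool helper loops Split to break strings into arrays, but nothing here calls it.
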(event `initializeGame`
  (bind _returnvalue (`KismetStringLibrary.Concat_StrStr` (`KismetStringLibrary.Replace` (`BlueprintPathsLibrary.GetProjectFilePath`) "/ProjectGroovy.uproject") "/Content/Data/test_song.json"))
  (if (not (`self.baseInitalized`))
    (set `self.baseInitalized` true)
    (`KismetSystemLibrary.PrintString` _returnvalue)
    (bind (_outjsonobject _returnvalue_2) (`JsonBlueprintFunctionLibrary.FromFile` (make `FilePath` _returnvalue)))
    (if _returnvalue_2
      (bind _outvalue (`|GetJsonField` _outjsonobject "BPM"))
      (bind _output_get (set `self.BPM` _outvalue))
      (`KismetSystemLibrary.PrintString` (`KismetStringLibrary.Conv_IntToString` _output_get))
      (bind _outvalue_2 (`|GetJsonField` _outjsonobject "Song"))
      (set `self.noteArray` _outvalue_2)
      (else
        (`KismetSystemLibrary.PrintString` "Failed to load JSON file")
        (`KismetSystemLibrary.Delay` 3.0)
        (`KismetSystemLibrary.QuitGame` null "Quit")))))

(fn `splitCool`
  (params (str :type String) (delimeter :type String))
  (returns (strArray :type "Array of String"))
  (bind _strarray (`self.strArray`))
  (bind (_lefts _rights _returnvalue) (`KismetStringLibrary.Split` (`self.tempStr`) delimeter))
  (set `self.tempStr` str)
  (while _returnvalue
    (set `self.tempStr` _rights)
    (`KismetArrayLibrary.Array_Add` _strarray _lefts))
  (`KismetArrayLibrary.Array_Add` _strarray _rights)
  (`KismetArrayLibrary.Array_Remove` _strarray (- (`KismetArrayLibrary.Array_Length` _strarray) 2))
  (return _strarray))

(fn `UserConstructionScript`)