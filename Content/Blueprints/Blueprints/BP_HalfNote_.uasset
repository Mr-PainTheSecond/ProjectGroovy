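; BP_HalfNote_ is a half-note actor for the rhythm game that configures itself on BeginPlay.
; It busy-loops until BP_RhythmGameMode is initialized, takes the next NoteArray entry as its index and advances SongIndex.
; That index picks its materials and bounds-scaled Y offset, while BPM and BaseMovement come from BP_NotePad.
; It also caches BP_Notes and the timing hitboxes as scoring actors; movement and scoring logic are absent here.
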(event `self.ReceiveBeginPlay`
  (bind _returnvalue (`self.GetTransform`))
  (bind _noteindex (`self.noteIndex`))
  ; Variable Initialization
  (bind _returnvalue_2 (`GameplayStatics.GetActorOfClass` "/Game/Blueprints/Blueprints/BP_RhythmGameMode.BP_RhythmGameMode_C"))
  (set `self.ready` (`/Game/Blueprints/Blueprints/BP_RhythmGameMode.baseInitalized` _returnvalue_2))
  (while (not (`self.ready`))
    (bind _returnvalue_3 (`GameplayStatics.GetActorOfClass` "/Game/Blueprints/Blueprints/BP_RhythmGameMode.BP_RhythmGameMode_C"))
    (set `self.ready` (`/Game/Blueprints/Blueprints/BP_RhythmGameMode.baseInitalized` _returnvalue_3)))
  (bind _returnvalue_4 (`GameplayStatics.GetActorOfClass` "/Game/Blueprints/Blueprints/BP_NotePad.BP_NotePad_C"))
  (bind _songindex (`/Game/Blueprints/Blueprints/BP_RhythmGameMode.songIndex` _returnvalue_2))
  (set `self.noteIndex` (`KismetStringLibrary.Conv_StringToInt` (`|GetArrayItem` (`/Game/Blueprints/Blueprints/BP_RhythmGameMode.noteArray` _returnvalue_2) _songindex)))
  (set `/Game/Blueprints/Blueprints/BP_RhythmGameMode.songIndex` (+ _songindex 1) _returnvalue_2)
  (set `self.baseMovement` (`/Game/Blueprints/Blueprints/BP_NotePad.baseMovement` _returnvalue_4))
  (set `self.BPM` (`/Game/Blueprints/Blueprints/BP_NotePad.BPM` _returnvalue_4))
  ;[0.05098 0.05098 0.05098] Sets up the positions and colors for the notes
  (bind (_center _boxextent) (`GameplayStatics.GetActorArrayBounds` (`|MakeArray` self :!type "Actor Object Reference")))
  (`PrimitiveComponent.SetMaterial` (`self.StaticMesh`) 0 (`|GetArrayItem` (`|MakeArray` (`self.yellow`) (`self.blue`) (`self.green`) (`self.red`)) _noteindex))
  (`PrimitiveComponent.SetMaterial` (`self.m&mCylinder`) 0 (`|GetArrayItem` (`self.materialGirls`) _noteindex))
  (`self.K2_SetActorLocation` (`KismetMathLibrary.MakeVector` (.x (`KismetMathLibrary.TransformLocation` _returnvalue)) (.y (`KismetMathLibrary.TransformLocation` _returnvalue (* (`KismetMathLibrary.MakeVector` 0.0 (.y _boxextent)) (`|GetArrayItem` (`|MakeArray` 0.0 0.086 0.172 0.258) (`self.noteIndex`))))) (.z (`KismetMathLibrary.TransformLocation` _returnvalue))))
  ; Creates an array which stores all the actors that are responsible for determining scoring when a note is played
  (bind _returnvalue_5 (`GameplayStatics.GetActorOfClass` "/Game/Blueprints/Blueprints/BP_Notes.BP_Notes_C"))
  (bind _output_get (set `self.allNoteScoreActors` (`|MakeArray` _returnvalue_5 :!type "Actor Object Reference")))
  (bind _outactors (`GameplayStatics.GetAllActorsOfClass` "/Game/Blueprints/Blueprints/BP_GreatHitbox.BP_GreatHitbox_C"))
  (for _array_element _outactors
    (`KismetArrayLibrary.Array_Add` _output_get _array_element))
  (bind _returnvalue_6 (`GameplayStatics.GetActorOfClass` "/Game/Blueprints/Blueprints/BP_GoodHitbox.BP_GoodHitbox_C"))
  (`KismetArrayLibrary.Array_Add` _output_get _returnvalue_6)
  (bind _returnvalue_7 (`GameplayStatics.GetActorOfClass` "/Game/Blueprints/Blueprints/BP_OKHitbox.BP_OKHitbox_C"))
  (`KismetArrayLibrary.Array_Add` _output_get _returnvalue_7)
  (bind _returnvalue_8 (`GameplayStatics.GetActorOfClass` "/Game/Blueprints/Blueprints/BP_EarlyHitbox.BP_EarlyHitbox_C"))
  (`KismetArrayLibrary.Array_Add` _output_get _returnvalue_8)
  (bind _returnvalue_9 (`GameplayStatics.GetActorOfClass` "/Game/Blueprints/Blueprints/BP_LateHitbox.BP_LateHitbox_C"))
  (`KismetArrayLibrary.Array_Add` _output_get _returnvalue_9))

(fn `UserConstructionScript`)