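; BP_NotePad is a scrolling segment of the rhythm game's note track that carries the song forward.
; On BeginPlay it steps along its length spawning BP_Beats measure bars and notes, choosing note types from markers in the game mode's NoteArray strings.
; Tick moves it at a BPM-scaled, frame-rate-independent speed unless the player is paused.
; Player overlap spawns the next pad at an offset, and BP_DeletePad overlaps destroy old pads.
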(event `self.ReceiveBeginPlay`
  (bind _rythmgameref (`self.rythmGameRef`))
  (bind _notearray (`/Game/Blueprints/Blueprints/BP_RhythmGameMode.noteArray` _rythmgameref))
  (bind _returnvalue (`KismetMathLibrary.TransformLocation` (`self.GetTransform`) (* (0.0 5.0 0.0) (`self.cubeOffsetScale`))))
  ; Variable Initialization
  (bind _returnvalue_2 (`GameplayStatics.GetActorOfClass` "/Game/Blueprints/Blueprints/BP_RhythmGameMode.BP_RhythmGameMode_C"))
  (set `self.barCount` (`/Game/Blueprints/Blueprints/BP_RhythmGameMode.quarterBeatCount` _returnvalue_2))
  (bind _returnvalue_3 (`GameplayStatics.GetActorOfClass` "/Game/Blueprints/Blueprints/BP_RhythmGameMode.BP_RhythmGameMode_C"))
  (`/Game/Blueprints/Blueprints/BP_RhythmGameMode.initializeGame` _returnvalue_3)
  (`self.K2_SetActorRotation` (`self.defaultRotations`))
  (bind _returnvalue_4 (`GameplayStatics.GetActorOfClass` "/Game/Blueprints/Blueprints/BP_RhythmGameMode.BP_RhythmGameMode_C"))
  (if (not (`/Game/Blueprints/Blueprints/BP_RhythmGameMode.firstNotePadCreated` _returnvalue_4))
    (set `self.first` true))
  (set `self.BPM` (`/Game/Blueprints/Blueprints/BP_RhythmGameMode.BPM` _returnvalue_4))
  (bind _output_get (set `self.startPOS` (`self.K2_GetActorLocation`)))
  (set `self.collided` false)
  (set `self.currentPOS` _output_get)
  (set `self.frames` 0.0)
  (bind _outactors (`GameplayStatics.GetAllActorsOfClass` "BP_NotePad_C"))
  (for _array_element _outactors
    (if (`/Game/Blueprints/Blueprints/BP_NotePad.spawning` _array_element)
      (set `self.newMeasureLocation` (mod (`KismetMathLibrary.Abs_Int` (`/Game/Blueprints/Blueprints/BP_NotePad.cubeOffsetScale` _array_element)) 100))
      (break)))
  ; Creates the measure bars and the notes which will be associated with this notepad
  (bind (_center _boxextent) (`GameplayStatics.GetActorArrayBounds` (`|MakeArray` self :!type "Actor Object Reference")))
  (set `self.outerBound` (+ (`self.startPOS`) _boxextent))
  (set `self.newBoxPOS` (`KismetMathLibrary.TransformLocation` (`self.GetTransform`) (* (0.0 5.0 0.0) (`KismetSystemLibrary.MakeLiteralInt` (`self.cubeOffsetScale`)))))
  (while (< (.z (`self.newBoxPOS`)) (+ (.z (`self.outerBound`)) -400.0))
    (if (== (mod (`KismetMathLibrary.Abs_Int` (`self.cubeOffsetScale`)) 100) (`self.newMeasureLocation`))
      (bind _returnvalue_5 (`|SpawnActorFromClass` "/Game/Blueprints/Blueprints/BP_Beats.BP_Beats_C" (`KismetMathLibrary.Conv_VectorToTransform` (`self.newBoxPOS`)) "Undefined" "MultiplyWithRoot" null null))
      (`self.K2_SetActorRotation` _returnvalue_5 (`self.defaultRotations`) false))
    (bind _returnvalue_6 (`GameplayStatics.GetActorOfClass` "/Game/Blueprints/Blueprints/BP_RhythmGameMode.BP_RhythmGameMode_C"))
    (set `self.rythmGameRef` _returnvalue_6)
    (if (and (not (`/Game/Blueprints/Blueprints/BP_RhythmGameMode.firstNotePadCreated` _returnvalue_6)) (< (`self.barCount`) 16))
      (set `self.barCount` (+ (`self.barCount`) 1) :!label _label)
      (set `self.cubeOffsetScale` (- (`self.cubeOffsetScale`) 25))
      (set `self.newBoxPOS` _returnvalue)
      (elif (>= (`/Game/Blueprints/Blueprints/BP_RhythmGameMode.songIndex` _rythmgameref) (`KismetArrayLibrary.Array_Length` _notearray))
        (goto _label)
        (elif (== (`KismetStringLibrary.Len` (`|GetArrayItem` _notearray (`/Game/Blueprints/Blueprints/BP_RhythmGameMode.songIndex` (`self.rythmGameRef`)))) 0)
          (set `/Game/Blueprints/Blueprints/BP_RhythmGameMode.songIndex` (+ (`/Game/Blueprints/Blueprints/BP_RhythmGameMode.songIndex` (`self.rythmGameRef`)) 1) (`self.rythmGameRef`))
          (set `self.cubeOffsetScale` (- (`self.cubeOffsetScale`) 25))
          (set `self.newBoxPOS` _returnvalue)
          (set `self.barCount` (+ (`self.barCount`) 1))
          (else
            (`self.noteControl`))))))
  (bind _returnvalue_7 (`GameplayStatics.GetActorOfClass` "/Game/Blueprints/Blueprints/BP_RhythmGameMode.BP_RhythmGameMode_C"))
  (if (not (`/Game/Blueprints/Blueprints/BP_RhythmGameMode.firstNotePadCreated` _returnvalue_7))
    (set `/Game/Blueprints/Blueprints/BP_RhythmGameMode.firstNotePadCreated` true _returnvalue_7)))

(event `self.ReceiveActorEndOverlap`
  (params (OtherActor :type "Actor Object Reference"))
  (cast `/Game/Blueprints/Blueprints/BP_DeletePad` OtherActor)
  (`self.K2_DestroyActor`))

(event `self.ReceiveActorBeginOverlap`
  (params (OtherActor :type "Actor Object Reference"))
  (bind _collided (`self.collided`))
  ; Handles the creations and destruction of this actor
  (cast `/Game/Blueprints/Blueprints/BP_FirstPersonCharacter` OtherActor
    (:`then`
      (set `self.spawning` true)
      (bind (_center _boxextent) (`GameplayStatics.GetActorArrayBounds` (`|MakeArray` self :!type "Actor Object Reference")))
      (if (`self.first`)
        (set `self.barNoteOffset` -1515)
        (else
          (set `self.barNoteOffset` -1400)))
      (bind _returnvalue (`|SpawnActorFromClass` "BP_NotePad_C" (`KismetMathLibrary.Conv_VectorToTransform` (`KismetMathLibrary.TransformLocation` (`self.GetTransform`) (* (0.0 5.0 0.0) (`KismetSystemLibrary.MakeLiteralInt` (`self.barNoteOffset`))))) "Undefined" "MultiplyWithRoot" null null))
      (`self.K2_SetActorRotation` _returnvalue (`self.K2_GetActorRotation`) false)
      (`self.setScale` _returnvalue))
    (:`CastFailed`
      (cast `/Game/Blueprints/Blueprints/BP_DeletePad` OtherActor)
      (`KismetSystemLibrary.PrintString` (`KismetStringLibrary.Conv_BoolToString` _collided))
      (if _collided
        (`self.K2_DestroyActor`)
        (else
          (set `self.collided` true))))))

(event `noteControl`
  (bind _songindex (`/Game/Blueprints/Blueprints/BP_RhythmGameMode.songIndex` (`self.rythmGameRef`)))
  (bind _notearray (`/Game/Blueprints/Blueprints/BP_RhythmGameMode.noteArray` (`self.rythmGameRef`)))
  (bind _output (`|GetArrayItem` (`/Game/Blueprints/Blueprints/BP_RhythmGameMode.noteArray` (`self.rythmGameRef`)) (`/Game/Blueprints/Blueprints/BP_RhythmGameMode.songIndex` (`self.rythmGameRef`))))
  (bind _returnvalue (`KismetStringLibrary.GetSubstring` _output))
  ; If the loop from BeginPlay reaches here, it is gurarantee that we are making a note. This section is in charge of determining what note is being created
  (set `self.fullNoteStr` _output)
  (if (!= -1 (`KismetStringLibrary.FindSubstring` _output "/"))
    (`KismetArrayLibrary.Array_Set` _notearray _songindex _returnvalue)
    (`self.createNote` "/Game/Blueprints/Blueprints/BP_QuaterNote.BP_QuaterNote_C")
    (elif (!= -1 (`KismetStringLibrary.FindSubstring` _output "?"))
      (`KismetArrayLibrary.Array_Set` _notearray _songindex _returnvalue)
      (`self.createNote` "/Game/Blueprints/Blueprints/BP_HalfNote_.BP_HalfNote__C")
      (elif (!= -1 (`KismetStringLibrary.FindSubstring` _output "L"))
        (`KismetArrayLibrary.Array_Set` _notearray _songindex _returnvalue)
        (`self.createNote` "/Game/Blueprints/Blueprints/BP_WholeNote.BP_WholeNote_C")
        (else
          (`self.createNote` "/Game/Blueprints/Blueprints/BP_PlayNotes.BP_PlayNotes_C"))))))

(event `self.ReceiveTick`
  (params (DeltaSeconds :type "Float (single-precision)"))
  (bind _returnvalue (`KismetMathLibrary.TransformLocation` (`self.GetTransform`) (* DeltaSeconds (* (`self.BPM`) (`self.baseMovement`)))))
  ; Moves note along the screen. Speed dependent on BPM, but independent of FPS
  (bind _returnvalue_2 (`GameplayStatics.GetActorOfClass` "/Game/Blueprints/Blueprints/BP_FirstPersonCharacter.BP_FirstPersonCharacter_C"))
  (if (not (`/Game/Blueprints/Blueprints/BP_FirstPersonCharacter.paused` _returnvalue_2))
    (`self.K2_SetActorLocation` _returnvalue)
    (set `self.currentPOS` _returnvalue)
    (set `self.frames` (+ (`self.frames`) 1.0))))

(event `setScale`
  ; Handles the creations and destruction of this actor
  (set `self.scale` 0.0))

(fn `createNote`
  (params (noteType :type "Actor Class Reference"))
  (bind _returnvalue (`|SpawnActorFromClass` noteType (`KismetMathLibrary.Conv_VectorToTransform` (`self.newBoxPOS`)) "AlwaysSpawn" "MultiplyWithRoot" null null))
  (bind _asbp_quater_note (cast `/Game/Blueprints/Blueprints/BP_QuaterNote` _returnvalue)
    (:`then`
      (set `/Game/Blueprints/Blueprints/BP_QuaterNote.quarterBeat` (`self.barCount`) _asbp_quater_note))
    (:`CastFailed`
      _))
  (`self.K2_SetActorRotation` _returnvalue (`self.defaultRotations`) false)
  (if (or (>= (`self.notesInMeasure`) 4) (!= (`KismetStringLibrary.FindSubstring` (`self.fullNoteStr`) ";") -1))
    (set `self.barCount` (+ (`self.barCount`) 1))
    (set `self.cubeOffsetScale` (- (`self.cubeOffsetScale`) 25))
    (set `self.newBoxPOS` (`KismetMathLibrary.TransformLocation` (`self.GetTransform`) (* (0.0 5.0 0.0) (`KismetSystemLibrary.MakeLiteralInt` (`self.cubeOffsetScale`)))))
    (set `self.notesInMeasure` 0)
    (else
      (set `self.notesInMeasure` (+ (`self.notesInMeasure`) 1)))))

(fn `UserConstructionScript`)