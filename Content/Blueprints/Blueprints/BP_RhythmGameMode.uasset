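; Rhythm game mode Blueprint that loads a song chart and prepares its scoring and end-of-song timing.
; On initialization it reads BPM, note strings and audio name from a hard-coded JSON file, quitting on failure.
; It totals the highest potential score using note-type values and combo-tier multipliers.
; After async-loading the SoundWave, it sets an end countdown from the final note's symbols; SplitCool is a string-splitting helper.
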(event `initializeGame`
  (bind _returnvalue (`KismetStringLibrary.Concat_StrStr` (`KismetStringLibrary.Replace` (`BlueprintPathsLibrary.GetProjectFilePath`) "/ProjectGroovy.uproject") "/Content/Data/billie_song.json"))
  (`KismetSystemLibrary.PrintString` "Game Start")
  (if (not (`self.baseInitalized`))
    (set `self.baseInitalized` true)
    (`KismetSystemLibrary.PrintString` _returnvalue)
    (bind (_outjsonobject _returnvalue_2) (`JsonBlueprintFunctionLibrary.FromFile` (make `FilePath` _returnvalue)))
    (if _returnvalue_2
      (bind _outvalue (`|GetJsonField` _outjsonobject "BPM"))
      (bind _output_get (set `self.BPM` _outvalue))
      (`KismetSystemLibrary.PrintString` (`KismetStringLibrary.Conv_IntToString` _output_get))
      (bind _outvalue_2 (`|GetJsonField` _outjsonobject "Song"))
      (set `self.noteArray` _outvalue_2)
      (`self.calculateHighestScore`)
      (bind _outvalue_3 (`|GetJsonField` _outjsonobject "mp3"))
      (bind _returnvalue_3 (`KismetSystemLibrary.Conv_SoftObjPathToSoftObjRef` (`KismetSystemLibrary.MakeSoftObjectPath` (`KismetStringLibrary.Concat_StrStr` "/Game/Songs/" _outvalue_3))))
      (if (not (`KismetSystemLibrary.IsValidSoftObjectReference` _returnvalue_3))
        (`KismetSystemLibrary.PrintString` "Not valid lol"))
      (bind _object (`|LoadAsset` _returnvalue_3)
        (:`Completed`
          (bind _assound_wave (cast `SoundWave` _object))
          (set `self.song` _assound_wave)
          (`self.finalCountdownSetup`)
          (set `self.finalBeat` -1)))
      (else
        (`KismetSystemLibrary.PrintString` "Failed to load JSON file")
        (`KismetSystemLibrary.Delay` 3.0)
        (`KismetSystemLibrary.QuitGame` null "Quit")))))

(event `calculateHighestScore`
  (for _array_element (`self.noteArray`)
    (if (!= (`KismetStringLibrary.Len` _array_element) 0)
      (set `self.noteCount` (+ (`self.noteCount`) 1))
      (if (>= (`self.noteCount`) 30)
        (set `self.multiplier` 8)
        (elif (>= (`self.noteCount`) 15)
          (set `self.multiplier` 4)
          (elif (>= (`self.noteCount`) 5)
            (set `self.multiplier` 2)
            (else
              (set `self.multiplier` 1)))))
      (if (and (== (`KismetStringLibrary.FindSubstring` _array_element "L") -1) (and (== (`KismetStringLibrary.FindSubstring` _array_element "?") -1) (== (`KismetStringLibrary.FindSubstring` _array_element "/") -1)))
        (set `self.highestPotentialScore` (+ (* 1000 (`self.multiplier`)) (`self.highestPotentialScore`)))
        (else
          (set `self.highestPotentialScore` (+ (* 2500 (`self.multiplier`)) (`self.highestPotentialScore`)))))))
  (`KismetSystemLibrary.PrintString` (`KismetStringLibrary.Conv_IntToString` (`self.highestPotentialScore`))))

(event `finalCountdownSetup`
  (bind _output_get (set `self.finalNote` (`|GetArrayItem` (`self.noteArray`) (- (`KismetArrayLibrary.Array_Length` (`self.noteArray`)) 1))))
  (if (== (`KismetStringLibrary.Len` _output_get) 1)
    (set `self.endCountdown` 16)
    (elif (!= (`KismetStringLibrary.FindSubstring` (`self.finalNote`) "/") -1)
      (set `self.endCountdown` 20)
      (elif (!= (`KismetStringLibrary.FindSubstring` (`self.finalNote`) "?") -1)
        (set `self.endCountdown` 24)
        (elif (!= (`KismetStringLibrary.FindSubstring` (`self.finalNote`) "L") -1)
          (set `self.endCountdown` 32)
          (else
            (set `self.endCountdown` 20)))))))

(fn `splitCool`
  (params (str :type String) (delimeter :type String))
  (returns (strArray :type "Array of String"))
  (bind _strarray (`self.strArray`))
  (bind (_lefts _rights _returnvalue) (`KismetStringLibrary.Split` (`self.tempStr`) delimeter))
  (set `self.tempStr` str)
  (while _returnvalue
    (set `self.tempStr` _rights)
    (`KismetArrayLibrary.Array_Add` _strarray _lefts))
  (`KismetArrayLibrary.Array_Add` _strarray _rights)
  (`KismetArrayLibrary.Array_Remove` _strarray (- (`KismetArrayLibrary.Array_Length` _strarray) 2))
  (return _strarray))

(fn `UserConstructionScript`)